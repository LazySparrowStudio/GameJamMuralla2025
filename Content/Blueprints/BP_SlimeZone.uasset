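; BP_SlimeZone is a trigger zone that completes once enough slimes of an accepted class have entered it.
; Box overlaps by that exact class increment a counter, which is never decremented, and set IsCompleted at the target amount.
; Tick watches that flag and fires OnZoneCompleted through a DoOnce.
; On BeginPlay, the Plane copies the mesh material of a found slime of the accepted class.
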(event OnComponentBeginOverlap(Box)
  (params (OverlappedComponent :type Primitive%20Component%20Object%20Reference) (OtherActor :type Actor%20Object%20Reference) (OtherComp :type Primitive%20Component%20Object%20Reference) (OtherBodyIndex :type Integer) (bFromSweep :type Boolean) (SweepResult :type Hit%20Result%20Structure%20%28by%20ref%29))
  ;[0.15 0.15 0.15 0.5] Gestiona cantidad
  (Development|PrintString "Hello")
  (if (== (Utilities|GetClass OtherActor) (Variables|Default|GetAcceptedSlimeClass))
    (Math|Integer|IncrementInt (Variables|Default|GetSlimeCounter)
      (:%20%20
        (if (== (Variables|Default|GetSlimeCounter) (Variables|Default|GetSlimeAmountToBeCompleted))
          (Variables|Default|SetisCompleted true))))))

(event EventBeginPlay
  ;[0.15 0.15 0.15 0.5] Coge el material
  (bind _returnvalue (Actor|GetActorOfClass (Variables|Default|GetAcceptedSlimeClass)))
  (Rendering|Material|SetMaterial (Variables|Default|GetPlane) 0 (Rendering|Material|GetMaterial (Variables|/Game/Blueprints/BP_SmallSlime_Base.BP_SmallSlime_Base_C|GetMesh _returnvalue) 0)))

(event Collision|EventActorBeginOverlap
  (params (OtherActor :type Actor%20Object%20Reference)))

(event EventTick
  (params (DeltaSeconds :type Float%20%28single-precision%29))
  ;[0.15 0.15 0.15 0.5] Avisa de que esta lista
  (if (Variables|Default|GetisCompleted)
    (Utilities|FlowControl|DoOnce false
      (:Completed
        (Development|PrintString "ZonaLista")
        (Default|CallOnZoneCompleted)))))

(fn ConstructionScript)