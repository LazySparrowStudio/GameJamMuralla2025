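; BP_SmallSlime_Base is a base Blueprint for a small slime that moves from an initial state to a settled, collectible one.
; On the first mesh hit, guarded by HasHit, it prints a debug message, switches SlimeCurrentState and stops physics simulation.
; BecomeCollectible makes the same state and physics change and also applies the CP_Active collision profile; the hit event duplicates this logic without calling it or changing collision.
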(event OnComponentHit(Mesh)
  (params (HitComponent :type Primitive%20Component%20Object%20Reference) (OtherActor :type Actor%20Object%20Reference) (OtherComp :type Primitive%20Component%20Object%20Reference) (NormalImpulse :type Vector :default "0, 0, 0") (Hit :type Hit%20Result%20Structure%20%28by%20ref%29))
  (if (not (Variables|Default|GethasHit))
    (Development|PrintString "Me he pegado")
    (Variables|Default|SethasHit true)
    (Variables|Default|SetSlimeCurrentState "NewEnumerator1")
    (Physics|SetSimulatePhysics (Variables|Default|GetMesh) false)))

(event EventBeginPlay
  (Variables|Default|SetSlimeCurrentState "NewEnumerator0"))

(fn ConstructionScript)

(fn BecomeCollectible
  (bind _mesh (Variables|Default|GetMesh))
  (Variables|Default|SetSlimeCurrentState "NewEnumerator1")
  (Physics|SetSimulatePhysics _mesh false)
  (Collision|SetCollisionProfileName _mesh "CP_Active" true :!class /Script/Engine.PrimitiveComponent))