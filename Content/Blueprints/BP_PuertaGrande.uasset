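; BP_PuertaGrande is a big-door indicator that changes appearance once all of its required zones are completed.
; On BeginPlay it sets the Sphere to the DoorClosed material and binds one handler to each RequiredZones completion event.
; Each event increments a counter, and when it equals the array length the Sphere switches to MTL_PuertaGrande.
; The file changes only the material, with no movement or collision logic.
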(event Custom|OnAnyZoneCompleted
  (bind _result (Math|Integer|IncrementInt (Variables|Default|GetCompletedCounterBig))
    (:%20%20
      (if (== _result (Utilities|Array|Length (Variables|Default|GetRequiredZones)))
        (Rendering|Material|SetMaterial (Variables|Default|GetSphere) 0 "/Game/Materials/MTL_PuertaGrande.MTL_PuertaGrande")))))

(event EventBeginPlay
  (Rendering|Material|SetMaterial (Variables|Default|GetSphere) 0 "/Game/Materials/DoorClosed.DoorClosed")
  (for _array_element (Variables|Default|GetRequiredZones)
    (EventDispatchers|BindEventtoOnZoneCompleted _array_element (delegate Custom|OnAnyZoneCompleted))))

(fn ConstructionScript)