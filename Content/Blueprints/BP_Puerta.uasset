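; BP_Puerta is a door that visually switches from closed to open once all of its required zones are completed.
; On BeginPlay it applies the closed material and binds to the completion event of each zone in RequiredZones.
; Each completion increments a counter, and when that equals the number of zones the open material is applied.
; The graph changes only the door's material, with no movement or collision logic.
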(event Custom|OnAnyZoneCompleted
  (bind _result (Math|Integer|IncrementInt (Variables|Default|GetCompletedCounter))
    (:%20%20
      (if (== _result (Utilities|Array|Length (Variables|Default|GetRequiredZones)))
        (Rendering|Material|SetMaterial (Variables|Default|GetDoor) 0 "/Game/Materials/DoorOpened.DoorOpened")))))

(event EventBeginPlay
  (Rendering|Material|SetMaterial (Variables|Default|GetDoor) 0 "/Game/Materials/DoorClosed.DoorClosed")
  (for _array_element (Variables|Default|GetRequiredZones)
    (EventDispatchers|BindEventtoOnZoneCompleted _array_element (delegate Custom|OnAnyZoneCompleted))))

(fn ConstructionScript)